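; Charge enemy Blueprint that cycles through idle, charging and tired states using three booleans.
; Tick runs a 0.2-second Delay into UpdateState, which advances to the next state regardless of the player.
; The loop that steers toward the player on X and Y while charging is disconnected, as is the PrintBools debug call, so the enemy only changes flags.
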(event EventBeginPlay)

(event Collision|EventActorBeginOverlap
  (params (OtherActor :type Actor%20Object%20Reference)))

(event EventTick
  (params (DeltaSeconds :type Float%20%28single-precision%29))
  (Utilities|FlowControl|Delay 0.2)
  (CallFunction|UpdateState))

(fn ConstructionScript)

(fn PrintBools
  (Development|PrintString "idle")
  (Development|PrintString (Utilities|String|ToString(Boolean) (Variables|Default|GetisIdle)))
  (Development|PrintString "charge")
  (Development|PrintString (Utilities|String|ToString(Boolean) (Variables|Default|GetisCharging)))
  (Development|PrintString "tired")
  (Development|PrintString (Utilities|String|ToString(Boolean) (Variables|Default|GetisTired))))

(fn UpdateState
  (if (Variables|Default|GetisIdle)
    (Variables|Default|SetisIdle false)
    (Variables|Default|SetisCharging true)
    (elif (Variables|Default|GetisCharging)
      (Variables|Default|SetisCharging false)
      (Variables|Default|SetisTired true)
      (else
        (Variables|Default|SetisTired false)
        (Variables|Default|SetisIdle true)))))