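; Player character with flipbook sprite animation, directional movement, a melee attack and spells cast through music-key combos.
; Tick picks the flipbook from last direction and attack state, briefly enabling that direction's hitbox to destroy overlapped Enemy actors.
; Music keys fill a capped, timed buffer that is matched against WomboCombo sequences.
; Spells are rough: Fireball spawns PlayerSpell, Haste only tints the sprite, Lightningbolt and Empower both spawn an Enemy.
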(event OnComponentBeginOverlap(attackHitBoxRight)
  (params (OverlappedComponent :type Primitive%20Component%20Object%20Reference) (OtherActor :type Actor%20Object%20Reference) (OtherComp :type Primitive%20Component%20Object%20Reference) (OtherBodyIndex :type Integer) (bFromSweep :type Boolean) (SweepResult :type Hit%20Result%20Structure%20%28by%20ref%29))
  (Development|PrintString "right")
  (if (== (Utilities|GetClass OtherActor) "/Game/blueprints/enemy.enemy_C")
    (Actor|DestroyActor OtherActor)))

(event OnComponentBeginOverlap(attackHitBoxUp)
  (params (OverlappedComponent :type Primitive%20Component%20Object%20Reference) (OtherActor :type Actor%20Object%20Reference) (OtherComp :type Primitive%20Component%20Object%20Reference) (OtherBodyIndex :type Integer) (bFromSweep :type Boolean) (SweepResult :type Hit%20Result%20Structure%20%28by%20ref%29))
  (Development|PrintString "up")
  (if (== (Utilities|GetClass OtherActor) "/Game/blueprints/enemy.enemy_C")
    (Actor|DestroyActor OtherActor)))

(event OnComponentBeginOverlap(attackHitBoxLeft)
  (params (OverlappedComponent :type Primitive%20Component%20Object%20Reference) (OtherActor :type Actor%20Object%20Reference) (OtherComp :type Primitive%20Component%20Object%20Reference) (OtherBodyIndex :type Integer) (bFromSweep :type Boolean) (SweepResult :type Hit%20Result%20Structure%20%28by%20ref%29))
  (Development|PrintString "left")
  (if (== (Utilities|GetClass OtherActor) "/Game/blueprints/enemy.enemy_C")
    (Actor|DestroyActor OtherActor)))

(event OnComponentBeginOverlap(attackHitBoxDown)
  (params (OverlappedComponent :type Primitive%20Component%20Object%20Reference) (OtherActor :type Actor%20Object%20Reference) (OtherComp :type Primitive%20Component%20Object%20Reference) (OtherBodyIndex :type Integer) (bFromSweep :type Boolean) (SweepResult :type Hit%20Result%20Structure%20%28by%20ref%29))
  (Development|PrintString "down")
  (if (== (Utilities|GetClass OtherActor) "/Game/blueprints/enemy.enemy_C")
    (Actor|DestroyActor OtherActor)))

(event EventBeginPlay
  (Variables|/Script/Engine.PrimitiveComponent|SetbGenerateOverlapEvents (Variables|Default|GetattackHitBoxDown) false)
  (Variables|/Script/Engine.PrimitiveComponent|SetbGenerateOverlapEvents (Variables|Default|GetattackHitBoxRight) false)
  (Variables|/Script/Engine.PrimitiveComponent|SetbGenerateOverlapEvents (Variables|Default|GetattackHitBoxLeft) false)
  (Variables|/Script/Engine.PrimitiveComponent|SetbGenerateOverlapEvents (Variables|Default|GetattackHitBoxUp) false)
  (bind _returnvalue (UserInterface|CreateWidget "/Game/blueprints/HUD.HUD_C"))
  (bind _output_get (Variables|Default|SetHUD%20Reference _returnvalue))
  (UserInterface|Viewport|AddtoViewport _output_get 0))

(event Collision|EventActorBeginOverlap
  (params (OtherActor :type Actor%20Object%20Reference)))

(event EventTick
  (params (DeltaSeconds :type Float%20%28single-precision%29))
  (bind _attackhitboxup (Variables|Default|GetattackHitBoxUp))
  (bind _attackhitboxleft (Variables|Default|GetattackHitBoxLeft))
  (bind _attackhitboxdown (Variables|Default|GetattackHitBoxDown))
  (bind _lastmovement (Variables|Default|GetLastMovement))
  (bind _attackhitboxright (Variables|Default|GetattackHitBoxRight))
  (bind _returnvalue (Utilities|Select :Index _lastmovement :NewEnumerator0 _attackhitboxup :NewEnumerator1 _attackhitboxdown :NewEnumerator2 _attackhitboxleft :NewEnumerator3 _attackhitboxright))
  ;[1 1 1] Animates Player
  (Pawn|Character|SetAnimation)
  ;[1 1 1] Sets a delay so that attack animation can play
  (if (Variables|Default|GetisAttacking)
    (Variables|/Script/Engine.PrimitiveComponent|SetbGenerateOverlapEvents _returnvalue (Variables|Default|GetisAttacking))
    (Utilities|FlowControl|Delay 0.4)
    (bind _output_get (Variables|Default|SetisAttacking false))
    (Variables|/Script/Engine.PrimitiveComponent|SetbGenerateOverlapEvents _returnvalue _output_get))
  (CallFunction|TimedRemovefromBuffer)
  (CallFunction|UpdateHud))

(event Input|ActionEvents|InputActionAttack
  (params (Key :type Key%20Structure :default "AnyKey"))
  (bind _attackhitboxup (Variables|Default|GetattackHitBoxUp))
  (bind _attackhitboxleft (Variables|Default|GetattackHitBoxLeft))
  (bind _attackhitboxdown (Variables|Default|GetattackHitBoxDown))
  (bind _lastmovement (Variables|Default|GetLastMovement))
  (bind _attackhitboxright (Variables|Default|GetattackHitBoxRight))
  (bind _returnvalue (Utilities|Select :Index _lastmovement :NewEnumerator0 _attackhitboxup :NewEnumerator1 _attackhitboxdown :NewEnumerator2 _attackhitboxleft :NewEnumerator3 _attackhitboxright))
  ;[1 1 1] Animates Attack
  (:Pressed
    (Variables|Default|SetisAttacking true)
    ;[1 1 1] Animates Player
    (Pawn|Character|SetAnimation)
    ;[1 1 1] Sets a delay so that attack animation can play
    (if (Variables|Default|GetisAttacking)
      (Variables|/Script/Engine.PrimitiveComponent|SetbGenerateOverlapEvents _returnvalue (Variables|Default|GetisAttacking))
      (Utilities|FlowControl|Delay 0.4)
      (bind _output_get (Variables|Default|SetisAttacking false))
      (Variables|/Script/Engine.PrimitiveComponent|SetbGenerateOverlapEvents _returnvalue _output_get))
    (CallFunction|TimedRemovefromBuffer)
    (CallFunction|UpdateHud)))

(event Input|ActionEvents|InputActionMusicUp
  (params (Key :type Key%20Structure :default "AnyKey"))
  (:Pressed
    (CallFunction|AddInput Key)
    (bind _didspecial (Pawn|Character|CheckCombos))
    (Variables|Default|SetdidSpecial false)
    (if _didspecial
      (switch Utilities|FlowControl|Switch|SwitchonComboEnum (Variables|Default|GetLastCombo)
        (:NewEnumerator0
          (Development|PrintString "LIGHTNINGBOLT")
          (AI|SpawnAIFromClass "/Game/blueprints/enemy.enemy_C" 0 "1.000000, 0, 0" "0, 0, 0" false :!label _label))
        (:NewEnumerator1
          (Development|PrintString "FIREBALL")
          (Game|SpawnActorfromClass "/Game/blueprints/playerSpell.playerSpell_C" (Math|Transform|MakeTransform (Transformation|GetActorLocation self)) "Undefined" 0 self))
        (:NewEnumerator2
          (Development|PrintString "HASTE")
          (Sprite|SetSpriteColor (Variables|Default|GetSprite) "(R=0.059657,G=0.999902,B=0.082216,A=1.000000)")
          (Physics|AddForce (Variables|Character|GetCharacterMovement) "0.000000,0.000000,0.000000"))
        (:NewEnumerator3
          (Development|PrintString "EMPOWER")
          (goto _label))))))

(event Input|ActionEvents|InputActionMusicDown
  (params (Key :type Key%20Structure :default "AnyKey"))
  (:Pressed
    (CallFunction|AddInput Key)
    (bind _didspecial (Pawn|Character|CheckCombos))
    (Variables|Default|SetdidSpecial false)
    (if _didspecial
      (switch Utilities|FlowControl|Switch|SwitchonComboEnum (Variables|Default|GetLastCombo)
        (:NewEnumerator0
          (Development|PrintString "LIGHTNINGBOLT")
          (AI|SpawnAIFromClass "/Game/blueprints/enemy.enemy_C" 0 "1.000000, 0, 0" "0, 0, 0" false :!label _label))
        (:NewEnumerator1
          (Development|PrintString "FIREBALL")
          (Game|SpawnActorfromClass "/Game/blueprints/playerSpell.playerSpell_C" (Math|Transform|MakeTransform (Transformation|GetActorLocation self)) "Undefined" 0 self))
        (:NewEnumerator2
          (Development|PrintString "HASTE")
          (Sprite|SetSpriteColor (Variables|Default|GetSprite) "(R=0.059657,G=0.999902,B=0.082216,A=1.000000)")
          (Physics|AddForce (Variables|Character|GetCharacterMovement) "0.000000,0.000000,0.000000"))
        (:NewEnumerator3
          (Development|PrintString "EMPOWER")
          (goto _label))))))

(event Input|ActionEvents|InputActionMusicLeft
  (params (Key :type Key%20Structure :default "AnyKey"))
  (:Pressed
    (CallFunction|AddInput Key)
    (bind _didspecial (Pawn|Character|CheckCombos))
    (Variables|Default|SetdidSpecial false)
    (if _didspecial
      (switch Utilities|FlowControl|Switch|SwitchonComboEnum (Variables|Default|GetLastCombo)
        (:NewEnumerator0
          (Development|PrintString "LIGHTNINGBOLT")
          (AI|SpawnAIFromClass "/Game/blueprints/enemy.enemy_C" 0 "1.000000, 0, 0" "0, 0, 0" false :!label _label))
        (:NewEnumerator1
          (Development|PrintString "FIREBALL")
          (Game|SpawnActorfromClass "/Game/blueprints/playerSpell.playerSpell_C" (Math|Transform|MakeTransform (Transformation|GetActorLocation self)) "Undefined" 0 self))
        (:NewEnumerator2
          (Development|PrintString "HASTE")
          (Sprite|SetSpriteColor (Variables|Default|GetSprite) "(R=0.059657,G=0.999902,B=0.082216,A=1.000000)")
          (Physics|AddForce (Variables|Character|GetCharacterMovement) "0.000000,0.000000,0.000000"))
        (:NewEnumerator3
          (Development|PrintString "EMPOWER")
          (goto _label))))))

(event Input|ActionEvents|InputActionMusicRight
  (params (Key :type Key%20Structure :default "AnyKey"))
  (:Pressed
    (CallFunction|AddInput Key)
    (bind _didspecial (Pawn|Character|CheckCombos))
    (Variables|Default|SetdidSpecial false)
    (if _didspecial
      (switch Utilities|FlowControl|Switch|SwitchonComboEnum (Variables|Default|GetLastCombo)
        (:NewEnumerator0
          (Development|PrintString "LIGHTNINGBOLT")
          (AI|SpawnAIFromClass "/Game/blueprints/enemy.enemy_C" 0 "1.000000, 0, 0" "0, 0, 0" false :!label _label))
        (:NewEnumerator1
          (Development|PrintString "FIREBALL")
          (Game|SpawnActorfromClass "/Game/blueprints/playerSpell.playerSpell_C" (Math|Transform|MakeTransform (Transformation|GetActorLocation self)) "Undefined" 0 self))
        (:NewEnumerator2
          (Development|PrintString "HASTE")
          (Sprite|SetSpriteColor (Variables|Default|GetSprite) "(R=0.059657,G=0.999902,B=0.082216,A=1.000000)")
          (Physics|AddForce (Variables|Character|GetCharacterMovement) "0.000000,0.000000,0.000000"))
        (:NewEnumerator3
          (Development|PrintString "EMPOWER")
          (goto _label))))))

(event Input|AxisEvents|InputAxisMovePlayerV
  (params (AxisValue :type Float%20%28single-precision%29))
  ;[1 1 1] Moves the player
  (Pawn|Input|AddMovementInput "0.000000,1.000000, 0" AxisValue false))

(event Input|AxisEvents|InputAxisMovePlayerH
  (params (AxisValue :type Float%20%28single-precision%29))
  ;[1 1 1] Moves the player
  (Pawn|Input|AddMovementInput "1.000000,0.000000,0.000000" AxisValue false))

(fn ConstructionScript)

(fn SetAnimation
  ;[1 1 1] will set the flipboook to dead if hp <=0, don't have death anim so sets to floor
  (if (Variables|Default|GetisDead)
    _
    (else
      _))
  (if (or (!= (Input|AxisValues|GetMovePlayerV) 0.0) (!= (Input|AxisValues|GetMovePlayerH) 0.0))
    (if (Variables|Default|GetisAttacking)
      _
      (else
        (Variables|Default|SetLastMovement (select (> (Input|AxisValues|GetMovePlayerV) 0.0) "NewEnumerator1" (select (< (Input|AxisValues|GetMovePlayerV) 0.0) "NewEnumerator0" (select (> (Input|AxisValues|GetMovePlayerH) 0.0) "NewEnumerator3" "NewEnumerator2")))))))
  (Sprite|SetFlipbook (Variables|Default|GetSprite) (select (Variables|Default|GetisAttacking) (Utilities|Select :Index (Variables|Default|GetLastMovement) :NewEnumerator0 "/Game/FlipBooks/attackUp.attackUp" :NewEnumerator1 "/Game/FlipBooks/attackDown.attackDown" :NewEnumerator2 "/Game/FlipBooks/attackLeft.attackLeft" :NewEnumerator3 "/Game/FlipBooks/attackRight.attackRight") (select (> (Math|Vector|VectorLength (Transformation|GetVelocity)) 0.0) (Utilities|Select :Index (Variables|Default|GetLastMovement) :NewEnumerator0 "/Game/FlipBooks/walkUp.walkUp" :NewEnumerator1 "/Game/FlipBooks/downWalk.downWalk" :NewEnumerator2 "/Game/FlipBooks/walkLeft.walkLeft" :NewEnumerator3 "/Game/FlipBooks/walkRight.walkRight") (Utilities|Select :Index (Variables|Default|GetLastMovement) :NewEnumerator0 "/Game/FlipBooks/standUp.standUp" :NewEnumerator1 "/Game/FlipBooks/standDown.standDown" :NewEnumerator2 "/Game/FlipBooks/standLeft.standLeft" :NewEnumerator3 "/Game/FlipBooks/standRight.standRight")))))

(fn AddInput
  (params (button :type Key%20Structure :default "AnyKey"))
  (bind _inputstiming (Variables|Default|GetInputsTiming))
  (bind _inputs (Variables|Default|GetInputs))
  (if (>= (Utilities|Array|Length _inputs) 9)
    (Utilities|Array|RemoveIndex _inputs)
    (Utilities|Array|RemoveIndex _inputstiming))
  (Utilities|Array|Add _inputs button)
  (Utilities|Array|Add _inputstiming (Math|DateTime|Now)))

(fn LoseHP
  (params (damage :type Integer))
  (bind _output_get (Variables|Default|SetHP (- (Variables|Default|GetHP) damage)))
  (Math|Integer|CompareInt (Variables|Default|GetHP) 0
    (:==
      _)
    (:<
      _))
  (Variables|Default|SetisDead true)
  (Development|PrintString (Utilities|String|ToString(Integer) _output_get)))

(fn MusicSpecial
  (params (ComboArray :type Array%20of%20Key%20Structures))
  (for (_array_element _array_index) (Variables|Default|GetInputs)
    (if (== _array_element (Utilities|Array|Get(acopy) ComboArray))
      (Variables|Default|SetdoSpecial false)
      (bind (_array_element_2 _array_index_2) (Utilities|Array|ForEachLoopwithBreak ComboArray)
        (:LoopBody
          (if (== _array_element_2 (Utilities|Array|Get(acopy) (Variables|Default|GetInputs) (+ _array_index_2 _array_index)))
            (Variables|Default|SetdoSpecial true)
            (else
              (Variables|Default|SetdoSpecial false)
              (return false))))
        (:Completed
          (if (Variables|Default|GetdoSpecial)
            (Variables|Default|SetdoSpecial false)
            (Utilities|Array|Clear (Variables|Default|GetInputs))
            (Utilities|Array|Clear (Variables|Default|GetInputsTiming))
            (return true)
            (else
              (return false)))))))
  (if (Variables|Default|GetdoSpecial)
    (Variables|Default|SetdoSpecial false)
    (Utilities|Array|Clear (Variables|Default|GetInputs))
    (Utilities|Array|Clear (Variables|Default|GetInputsTiming))
    (return true)
    (else
      (return false))))

(fn CheckCombos
  (for (_array_element _array_index) (Variables|Default|GetwomboCombo)
    (bind _didspecial (Pawn|Character|MusicSpecial (Utilities|Struct|BreakCombo _array_element)))
    (if _didspecial
      (switch int _array_index
        (:0
          (Variables|Default|SetLastCombo "NewEnumerator0"))
        (:1
          (Variables|Default|SetLastCombo "NewEnumerator1"))
        (:2
          (Variables|Default|SetLastCombo "NewEnumerator2"))
        (:3
          (Variables|Default|SetLastCombo "NewEnumerator3")))
      (Variables|Default|SetdidSpecial true)))
  (return (Variables|Default|GetdidSpecial)))

(fn UpdateHud
  (bind _inputs (Variables|Default|GetInputs))
  (Variables|Default|SetstrInputs "")
  (for _index (range 0 (- (Utilities|Array|Length _inputs) 1))
    (Variables|Default|SetstrInputs (Utilities|String|Append (Variables|Default|GetstrInputs) (Utilities|String|ToString(Text) (Class|KismetInputLibrary|KeyGetDisplayName (Utilities|Array|Get(acopy) _inputs _index)))))))

(fn TimedRemovefromBuffer
  (bind _inputstiming (Variables|Default|GetInputsTiming))
  (if (> (Utilities|Array|Length _inputstiming) 0)
    (if (< (Utilities|Array|Get(acopy) _inputstiming) (- (Math|DateTime|Now) (Math|Timespan|MakeTimespan 0 0 0 5)))
      (Utilities|Array|RemoveIndex _inputstiming)
      (Utilities|Array|RemoveIndex (Variables|Default|GetInputs)))))