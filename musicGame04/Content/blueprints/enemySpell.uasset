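; Enemy fireball spell actor that damages the player on overlap.
; On BeginPlay it reads the player's LastMovement and adds a projectile movement component per direction, intended to fire where the player faces, though a comment marks this as broken.
; Overlapping a Player calls LoseHP with its Damage and prints a debug message.
; An unconnected look-at rotation is an unfinished attempt to aim at the player instead.
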(event EventTick
  (params (DeltaSeconds :type Float%20%28single-precision%29)))

(event EventBeginPlay
  ;[1 1 1] broken POS that has the fireball shoot in the directon the player is facing
  (bind _asplayer (Utilities|Casting|CastToPlayer (Game|GetPlayerCharacter 0)))
  (Variables|Default|SetMy%20Character _asplayer)
  (switch Utilities|FlowControl|Switch|SwitchonMovement (Variables|/Game/blueprints/Player.Player_C|GetLastMovement (Variables|Default|GetMy%20Character))
    (:NewEnumerator0
      (AddComponent|AddProjectileMovementComponent))
    (:NewEnumerator1
      (AddComponent|AddProjectileMovementComponent))
    (:NewEnumerator2
      (AddComponent|AddProjectileMovementComponent))
    (:NewEnumerator3
      (AddComponent|AddProjectileMovementComponent))))

(event Collision|EventActorBeginOverlap
  (params (OtherActor :type Actor%20Object%20Reference))
  ;[1 1 1] Enemy version to make the player take damage
  (if (== (Utilities|GetClass OtherActor) "/Game/blueprints/Player.Player_C")
    (bind _asplayer (Utilities|Casting|CastToPlayer (Game|Player|GetPlayerPawn 0))
      (:then
        (Default|LoseHP _asplayer (Variables|Default|Getdamage))
        (Development|PrintString "get fireballed kiddo"))
      (:CastFailed
        (Development|PrintString "shits fucked")))))

(fn ConstructionScript
  (|CallParentFunction))